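; Procedural walking leg component that computes a foot target and stepping motion for the owning character, updated by the Leg Manager.
; A fallback cascade of line, sphere and radial traces seeks footing ahead, beneath or, for non-bipeds, on walls.
; Distant targets trigger a replant, gated by the manager.
; Speed-timed, curve-driven steps write foot positions to the manager's LegInfo; falling resets feet to the component location.
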(event EventBeginPlay
  (bind _returnvalue (Components|GetOwner))
  (bind _returnvalue_2 (Actor|GetComponentbyClass _returnvalue "/Script/Engine.CapsuleComponent"))
  (bind _returnvalue_3 (Components|Capsule|GetScaledCapsuleHalfHeight _returnvalue_2))
  (bind _returnvalue_4 (Components|Capsule|GetScaledCapsuleRadius _returnvalue_2))
  ;[0 0 0] At start we're setting the Leg_Manager, the default foot position and the Trace height, which will be calculated by the capsule height which should be fine for most situations. Use the Add-Trace-Height variable to fine tune the trace height, for Bipeds you probably want to shorten it. Same goes for the Step-Length. We also set the Capsule-Radius/Height for later so we don't constantly have to call for it. We also need to preset the Plant-Start-Position otherwise our Character will start from the world origin location and move into position after spawning in. We also save the Character-Movement-Component to check for falling states.
  (Variables|Default|SetLeg%20Manager (Actor|GetComponentbyClass (Components|GetOwner) (Variables|LegSettings|GetBP%20Leg%20Manager%20Class)))
  (Variables|Internal|SetFoot%20Position (Transformation|GetWorldLocation))
  (Variables|Internal|SetTrace%20Height (+ _returnvalue_3 (Variables|LegSettings|GetAdd%20Trace%20Height)))
  (Variables|Internal|SetStep%20Length (+ _returnvalue_4 (Variables|LegSettings|GetAdd%20Step%20Length)))
  (Variables|Internal|SetStep%20Height (+ _returnvalue_3 (Variables|LegSettings|GetAdd%20Step%20Height)))
  (Variables|Internal|SetCapsule%20Radius _returnvalue_4)
  (Variables|Internal|SetCapsule%20Height _returnvalue_3)
  (Variables|Internal|SetPlant%20Start%20Position (Transformation|GetWorldLocation))
  (Variables|Default|SetCharacter%20Movement%20Component (Actor|GetComponentbyClass (Components|GetOwner) "/Script/Engine.CharacterMovementComponent")))

(fn UpdateFoot
  (params (Index :type Integer))
  (bind _returnvalue (Transformation|GetWorldLocation))
  ;[0 0 0] This is our basic loop, which will be called by the Leg-Manager to update the Foot position.
  (Variables|Internal|SetLeg_Count Index)
  (if (not (AI|Components|NavMovement|IsFalling (Variables|Default|GetCharacter%20Movement%20Component)))
    (UpdateFoot|GetFootTargetLocation)
    (UpdateFoot|CheckforReplant)
    (UpdateFoot|TakeFootStep)
    (else
      ;[0 0 0] In case the Character is falling/jumping we will stop all calculations. If you would like to keep the tracing going just remove the above Branch node.
      (Utilities|Array|SetArrayElem (Variables|/Game/Procedural_Walk_BPs/BP_Leg_Manager_V2.BP_Leg_Manager_V2_C|GetLeg_Info (Actor|GetComponentbyClass (Components|GetOwner) (Variables|LegSettings|GetBP%20Leg%20Manager%20Class))) (Variables|Internal|GetLeg_Count) _returnvalue true)
      (Variables|Internal|SetFoot%20Position _returnvalue)
      (Variables|Internal|SetIs%20Planted true))))

(fn GetFootTargetLocation
  (Utilities|FlowControl|Sequence
    (:then_0
      ;[0 0 0] To start with, we will get our Actors (to which this BP is attached to) Character-Movement-Component and from that we will need the Last-Input-Vector to get our movement direction in world space. Then we Normalize that direction and multiply it by the Step-Length which can be changed to whatever is needed. Now we have the direction and the distance, so we take our Actors up vector (which is dependent on our Actors overall rotation) and multiply that by the Trace-Height (which by default is the half height of our capsule). This gives us the elevation we need. Very important for traces is to not forget to add the current world location. So we add the Current World location to the elevation and add to that the direction and distance. This finally results in our Line-Trace starting position.
      (LocalVariables|SetRay%20Start (+ (+ (* (Transformation|GetActorUpVector (Components|GetOwner)) (Variables|Internal|GetTrace%20Height)) (Transformation|GetWorldLocation)) (* (Math|Vector|Normalize (Pawn|Components|PawnMovement|GetLastInputVector (Actor|GetComponentbyClass (Components|GetOwner) "/Script/Engine.CharacterMovementComponent"))) (Variables|Internal|GetStep%20Length)))))
    (:then_1
      ;[0 0 0] Next step we will use the Actors up vector again, negate it and multiply it by the double Trace_Height. This will give us the negative height, to which we will add the Ray-Start position to get the Ray-End position.
      (LocalVariables|SetRay%20End (+ (* (Math|Vector|NegateVector (Transformation|GetActorUpVector (Components|GetOwner))) (* (Variables|Internal|GetTrace%20Height) 2.0)) (LocalVariables|GetRay%20Start))))
    (:then_2
      ;[0 0 0] And now we will feed those positions into a series of different Traces to check for about every situation and try our hardest to find a ground to stand on. We will go trough them one by one and if on fails we will go to the next one. If a trace does find something it will set the traced position as the Target-Position and move on to the next step. This way we can avoid doing traces when they're not neccesarry. You can double click on either the trace macro or the collapsed graphs and i will explain them in there in more detail.
      (if (not (Variables|LegSettings|GetIs%20Biped))
        (bind _out_hit_location (Utilities|RadialWallTrace)
          (:Done
            (Variables|Internal|SetTarget%20Position _out_hit_location))
          (:false
            (|LineTrace1 :!label _label
              (:False
                (|LineTrace2
                  (:False
                    (|RadialTrace2
                      (:False
                        (|LineTrace3)))))))))
        (else
          (goto _label))))
    (:then_3
      ;[0 0 0] This is to visualize the calculated positions during gameplay.
      (if (Variables|LegSettings|GetDraw%20Debug%20Paths)
        (Rendering|Debug|DrawDebugBox (Variables|Internal|GetPlant%20Start%20Position) "10.000000,10.000000,10.000000" "(R=0.918135,G=0.000000,B=1.000000,A=1.000000)" "0, 0, 0" (Variables|Internal|GetStep%20Time) 0.0)
        (Rendering|Debug|DrawDebugBox (Variables|Internal|GetTarget%20Position) "10.000000,10.000000,10.000000" "(R=1.000000,G=0.441190,B=0.000000,A=1.000000)" "0, 0, 0" 0.0 0.0)
        (Rendering|Debug|DrawDebugLine (Variables|Internal|GetPlant%20Start%20Position) (Variables|Internal|GetTarget%20Position) "(R=1.000000,G=0.045259,B=0.000000,A=1.000000)" 0.0 1.0)
        (Rendering|Debug|DrawDebugBox (Variables|Internal|GetFoot%20Position) "15.000000,15.000000,15.000000" "(R=0.116241,G=1.000000,B=0.000000,A=1.000000)" "0, 0, 0" 0.0 0.0)))))

(fn CheckforReplant
  (Utilities|FlowControl|Sequence
    (:then_0
      ;[0 0 0] Here we check if it's worth replanting the foot. If the lengt between the Foot-Position and the Target-Position is big enough, it will try to replant unless it already is planted. This will remove unnecessary foot movement, and after stopping any movement it will relplant all legs to their base position if they're too far away, which looks and feels much more natural.
      (LocalVariables|SetWant%20To%20Replant (and (Variables|Internal|GetIs%20Planted) (> (Math|Vector|VectorLength (- (Variables|Internal|GetFoot%20Position) (Variables|Internal|GetTarget%20Position))) (Variables|Internal|GetCapsule%20Radius)))))
    (:then_1
      ;[0 0 0] If the Leg wants to replant, it will ask the Leg-Manager for permission. Only after having the leg wanting to replace and the Leg-Manager allowing it, we will set the leg to actually do the replant.
      (LocalVariables|SetDo%20Replant (and (LocalVariables|GetWant%20To%20Replant) (Default|CanLegUnplant (Variables|Default|GetLeg%20Manager) self))))
    (:then_2
      ;[0 0 0] If we do replant the leg, we set the leg as unplanted, set the current Foot-Position as the Plant-Start-Position for later use, and reset the Time-Since-Unplanted.
      (if (LocalVariables|GetDo%20Replant)
        (Utilities|FlowControl|Sequence
          (:then_0
            (Variables|Internal|SetIs%20Planted false))
          (:then_1
            (Variables|Internal|SetPlant%20Start%20Position (Variables|Internal|GetFoot%20Position)))
          (:then_2
            (Variables|Internal|SetTime%20Since%20Unplanted 0.0)))))))

(fn TakeFootStep
  (if (Variables|Internal|GetIs%20Planted)
    (return)
    (else
      (Utilities|FlowControl|Sequence
        (:then_0
          ;[0 0 0] Get the Character_BP's current max movement speed and divide it by the Step-Length multiplied by 2, so we get the max distance your foot will stay on the ground before it should replant again as to have a smooth walk-cycle. This will give us the amount of steps the Character can take in 1 second, since the Character_BP's movement speed is expressed in cm/s. So if we divide 1 Second by the steps per second we get the time it takes to make 1 step.
          (Variables|Internal|SetStep%20Time (/ 1.0 (/ (Class|MovementComponent|GetMaxSpeed (Actor|GetComponentbyClass (Components|GetOwner) "/Script/Engine.MovementComponent")) (* (Variables|Internal|GetStep%20Length) 2.0)))))
        (:then_1
          ;[0 0 0] By dividing the Time-Since-Unplanted by the Step-Time we can track the progress of the step.
          (Variables|Internal|SetPercentage%20Replanted (/ (Variables|Internal|GetTime%20Since%20Unplanted) (Variables|Internal|GetStep%20Time))))
        (:then_2
          ;[0 0 0] Now we lerp from the Plant-Start-Position towards the traced Target-Position and set it as the Foot-Position. Lerp chooses a point between A and B depending on the Alpha value (which goes from 0 to 1), so using the current step progression expressed in the Percentage-Replanted it will return the corresponding value of the curve. The curves give us better control of the foot movement. So we use the same method to get the height of the foot during replanting. Change the Step-Height to change the amount the foot will be lifted.
          (Variables|Internal|SetFoot%20Position (+ (Math|Vector|Lerp(Vector) (Variables|Internal|GetPlant%20Start%20Position) (Variables|Internal|GetTarget%20Position) (Math|Curves|GetFloatValue (LocalVariables|GetReplant%20Speed%20Curve) (Variables|Internal|GetPercentage%20Replanted))) (* (Transformation|GetActorUpVector (Components|GetOwner)) (- (* (Math|Curves|GetFloatValue (LocalVariables|GetReplant%20Height%20Curve) (Variables|Internal|GetPercentage%20Replanted)) (Variables|Internal|GetStep%20Height)) (Variables|LegSettings|GetFoot%20Offset)))))
          (Utilities|Array|SetArrayElem (Variables|/Game/Procedural_Walk_BPs/BP_Leg_Manager_V2.BP_Leg_Manager_V2_C|GetLeg_Info (Actor|GetComponentbyClass (Components|GetOwner) (Variables|LegSettings|GetBP%20Leg%20Manager%20Class))) (Variables|Internal|GetLeg_Count) (Variables|Internal|GetFoot%20Position) true))
        (:then_3
          ;[0 0 0] After that we will Add the current runtime to the Time-Since-Unplanted and set it as the new Time-Since-Unplanted. This way it will count up towards the Step-Time. As soon as the Time-Since-Unplanted is equal or greater than the Step-Time we will consider the step finished and we will let the Leg-Manager know.
          (Variables|Internal|SetTime%20Since%20Unplanted (+ (Variables|Internal|GetTime%20Since%20Unplanted) (Utilities|Time|GetWorldDeltaSeconds)))
          (Variables|Internal|SetIs%20Planted (>= (Variables|Internal|GetTime%20Since%20Unplanted) (Variables|Internal|GetStep%20Time))))))))